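; BP_Prop is a static mesh prop that can darken its appearance when play begins.
; On BeginPlay it creates a dynamic instance of the chicken colors material on its mesh, then calls Darken if the Dark flag is false.
; Darken lowers the red channel of the "darkness" vector parameter by a fixed step and writes the result back as a color.
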(event EventBeginPlay
  (bind _returnvalue (Rendering|Material|CreateDynamicMaterialInstance (Variables|Default|GetStaticMesh) 0 "/Game/media/meshes/M_chicken__colors_png.M_chicken__colors_png" "None" :!class /Script/Engine.PrimitiveComponent))
  (Variables|Default|SetMaterialInstance _returnvalue)
  (if (not (Variables|Default|GetDark))
    (CallFunction|Darken)))

(fn ConstructionScript)

(fn Darken
  (bind _materialinstance (Variables|Default|GetMaterialInstance))
  (bind _returnvalue (Rendering|Material|GetVectorParameterValue _materialinstance "darkness" :!class /Script/Engine.MaterialInstanceDynamic))
  (Rendering|Material|SetVectorParameterValue _materialinstance "darkness" (Math|Conversions|ToLinearColor(Float) (- (.R (Utilities|Struct|BreakLinearColor _returnvalue)) 0.4)) :!class /Script/Engine.MaterialInstanceDynamic))