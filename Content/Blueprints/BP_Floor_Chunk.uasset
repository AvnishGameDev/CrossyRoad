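; Floor chunk for a chicken game: one row of ground that owns left, center and right floor pieces, landing nodes and props.
; Helper functions compute the three floor transforms, spawn landing nodes stepped along X with a water flag, and randomly spawn coins.
; Each Tick it checks its Y against the chicken's and, once past the trailing distance limit, destroys its pieces, nodes, props and itself.
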(event EventTick
  (params (DeltaSeconds :type Float%20%28single-precision%29))
  (CallFunction|CheckifDestroyFloorChunk))

(fn ConstructionScript)

(fn CalculateFloorTransform
  (bind _positiony (Variables|Default|GetPositionY))
  (return (Math|Transform|MakeTransform (Math|Vector|MakeVector -1.8e+03 _positiony 0.0)) (Math|Transform|MakeTransform (Math|Vector|MakeVector 0.0 _positiony 0.0)) (Math|Transform|MakeTransform (Math|Vector|MakeVector 1.8e+03 _positiony 0.0)) _positiony))

(fn DestroyMeshesLandingNodesandProps
  (for _array_element (Variables|Default|GetLandingNodes)
    (Actor|DestroyActor _array_element))
  (Actor|DestroyActor (Variables|Default|GetLeftFloor))
  (Actor|DestroyActor (Variables|Default|GetRightFloor))
  (Actor|DestroyActor (Variables|Default|GetCenterFloor))
  (for _array_element_2 (Variables|Default|GetProps)
    (Actor|DestroyActor _array_element_2)))

(fn CheckifDestroyFloorChunk
  (bind _chickenref (Variables|Default|GetChickenRef))
  (Utilities|IsValid _chickenref
    (:Is%20Valid
      (if (>= (.y (Transformation|GetActorLocation)) (+ (.y (Transformation|GetActorLocation _chickenref)) (Variables|Default|GetMaxDistanceBackFromChicken)))
        (CallFunction|DestroyMeshesLandingNodesandProps)
        (Actor|DestroyActor)))))

(fn ContructLandingNode(FloorChunk)
  (params (bIsWater :type Boolean))
  (bind _returnvalue (Game|SpawnActorfromClass "/Game/Blueprints/BP_Landing_Node.BP_Landing_Node_C" (Math|Transform|MakeTransform (Math|Vector|MakeVector (Variables|Default|GetCurrentXPosForLandingNode) (.y (Transformation|GetActorLocation)) (Variables|Default|GetCurrentZPosForLandingNode))) "Undefined" 0 bIsWater 0))
  (Variables|Default|SetCurrentXPosForLandingNode (+ (Variables|Default|GetCurrentXPosForLandingNode) 2e+02))
  (Utilities|Array|Add (Variables|Default|GetLandingNodes) _returnvalue))

(fn CreateCoinAttempt
  (if (== (Math|Random|RandomInteger 9) 0)
    (Game|SpawnActorfromClass "/Game/Blueprints/BP_Coin.BP_Coin_C" (Math|Transform|MakeTransform (Math|Vector|MakeVector (Variables|Default|GetCurrentXPosForLandingNode) (.y (Transformation|GetActorLocation)) (Variables|Default|GetCurrentZPosForLandingNode))) "Undefined" 0 0)))