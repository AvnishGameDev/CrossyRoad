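; BP_Bounce is an actor Blueprint that animates a short vertical bounce when flagged as being jumped on.
; Tick advances a timer and, after a start delay, computes a Z offset from a hard-coded parabola, applied to a cached height.
; A reset clears the flag, timer and offset once the time window set on BeginPlay ends.
; The flag and cached height are not set in these graphs.
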(event EventBeginPlay
  (Variables|Default|SetMaximumJumpedOnTime (+ (Variables|Default|GetMaximumStartJumpTime) 0.2)))

(event EventTick
  (params (DeltaSeconds :type Float%20%28single-precision%29))
  (CallFunction|BouncingAnimation DeltaSeconds))

(fn ConstructionScript)

(fn ResetAnimation
  (Variables|Default|SetbIsBeingJumpedOn false)
  (Variables|Default|SetJumpedOnZOffset 0.0)
  (Variables|Default|SetCurrentJumpedOnTime 0.0))

(fn JumpedonAnimation
  (params (DeltaTime :type Float%20%28single-precision%29))
  (Variables|Default|SetCurrentJumpedOnTime (+ DeltaTime (Variables|Default|GetCurrentJumpedOnTime)))
  (if (>= (Variables|Default|GetCurrentJumpedOnTime) (Variables|Default|GetMaximumStartJumpTime))
    (if (>= (Variables|Default|GetCurrentJumpedOnTime) (Variables|Default|GetMaximumJumpedOnTime))
      (CallFunction|ResetAnimation)
      (else
        (Variables|Default|SetJumpedOnZOffset (* (- (Math|Float|Square (- (* (- (Variables|Default|GetCurrentJumpedOnTime) 0.1) 8.0) 1.0)) 1.0) 2e+01))))))

(fn BouncingAnimation
  (params (Delta%20Time :type Float%20%28single-precision%29))
  (bind _returnvalue (Transformation|GetActorLocation))
  (if (Variables|Default|GetbIsBeingJumpedOn)
    (CallFunction|JumpedonAnimation Delta%20Time)
    (Transformation|SetActorLocation (Math|Vector|MakeVector (.x _returnvalue) (.y _returnvalue) (+ (Variables|Default|GetCachedZPosition) (Variables|Default|GetJumpedOnZOffset))) false false)))