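; BP_Bush is a foliage prop actor that randomizes its look in the construction script, with no active gameplay logic.
; A random roll sets one of three quarter-turn rotations, then a second roll assigns one of three tree meshes to its StaticMesh.
; A zero on the first roll skips both steps, and a three on the second keeps the current mesh.
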(event EventBeginPlay
  (|CallParentFunction) ; This node is disabled and will not be called.\nDrag off pins to build functionality.
)

(event Collision|EventActorBeginOverlap
  (params (OtherActor :type Actor%20Object%20Reference)))

(event EventTick
  (params (DeltaSeconds :type Float%20%28single-precision%29)))

(fn ConstructionScript
  (bind _staticmesh (Variables|Default|GetStaticMesh))
  (|CallParentFunction)
  (switch int (Math|Random|RandomIntegerinRange 0 3)
    (:1
      (Transformation|SetActorRotation "0,90.000000, 0"))
    (:2
      (Transformation|SetActorRotation "0,180.000000, 0"))
    (:3
      (Transformation|SetActorRotation "0,270.000000, 0")))
  (switch int (Math|Random|RandomIntegerinRange 0 3)
    (:0
      (Components|StaticMesh|SetStaticMesh _staticmesh "/Game/media/meshes/tree1.tree1"))
    (:1
      (Components|StaticMesh|SetStaticMesh _staticmesh "/Game/media/meshes/tree2.tree2"))
    (:2
      (Components|StaticMesh|SetStaticMesh _staticmesh "/Game/media/meshes/tree3.tree3"))))