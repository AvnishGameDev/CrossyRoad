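; BP_Main_Camera is a camera actor that follows the player's chicken in a Crossy Road-style game.
; BeginPlay caches the player pawn as a BP_ChickenBase, then sets the ChickenRef on BP_GameMode_CrossyRoad to None.
; Tick moves the actor to the chicken's Y plus an offset, with X and height held fixed, so it tracks along one axis without smoothing.
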(event EventBeginPlay
  (bind _asbp_chicken (Utilities|Casting|CastToBP_ChickenBase (Game|Player|GetPlayerPawn 0)))
  (Variables|Default|SetChickenRef _asbp_chicken)
  (bind _asbp_game_mode_crossy_road (Utilities|Casting|CastToBP_GameMode_CrossyRoad (Game|GetGameMode)))
  (Variables|/Game/Blueprints/BP_GameMode_CrossyRoad.BP_GameMode_CrossyRoad_C|SetChickenRef _asbp_game_mode_crossy_road 0))

(event EventTick
  (params (DeltaSeconds :type Float%20%28single-precision%29))
  (Transformation|SetActorLocation (Math|Vector|MakeVector 0.0 (+ (.Y (Math|Vector|BreakVector (Transformation|GetActorLocation (Variables|Default|GetChickenRef)))) (Variables|Default|GetOffsetY)) 1.3e+03) false false))

(fn ConstructionScript)