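; BP_Train is a moving train hazard that ends the game for the chicken player on contact.
; Each tick it moves along world X at MoveSpeed, with MoveLeft reversing the direction and setting a 180-degree rotation at BeginPlay.
; A LifeTime countdown destroys the actor when it runs out.
; Any overlap with BP_Chicken_Player calls that player's GameOverSequence.
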(event EventBeginPlay
  (if (Variables|Default|GetbMoveLeft)
    (Transformation|SetActorRotation "0,180.000000, 0")))

(event Collision|EventActorBeginOverlap
  (params (OtherActor :type Actor%20Object%20Reference))
  (bind _asbp_chicken_player (Utilities|Casting|CastToBP_Chicken_Player OtherActor))
  (Default|GameOverSequence _asbp_chicken_player))

(event EventTick
  (params (DeltaSeconds :type Float%20%28single-precision%29))
  (bind _movespeed (Variables|Default|GetMoveSpeed))
  (bind _returnvalue (* DeltaSeconds _movespeed))
  (if (Variables|Default|GetbMoveLeft)
    (Transformation|AddActorWorldOffset (Math|Vector|MakeVector (* _returnvalue -1.0) 0.0 0.0))
    (else
      (Transformation|AddActorWorldOffset (Math|Vector|MakeVector _returnvalue 0.0 0.0))))
  (bind _output_get (Variables|Default|SetLifeTime (- (Variables|Default|GetLifeTime) DeltaSeconds)))
  (if (<= _output_get 0.0)
    (Actor|DestroyActor)))

(fn ConstructionScript)