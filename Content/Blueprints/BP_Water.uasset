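; BP_Water is a water-row floor chunk for a Frogger-style crossing game, with optional moving logs and lily pads.
; It spawns three floor sections and landing nodes, placing up to three lily pads at distinct clear-column positions.
; Logs pre-fill the row, then spawn from one side on a timer scaled by log length and the row's random speed bonus.
; Tick checks for chunk removal, and destruction removes its lily pads.
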(event EventBeginPlay
  (bind _self self)
  (bind (_transformleft _transformmid _transformright) (CallFunction|CalculateFloorTransform))
  (bind _returnvalue (Game|SpawnActorfromClass "/Game/Blueprints/BP_Floor.BP_Floor_C" _transformleft "Undefined" 0 2 false _self 0))
  (Variables|Default|SetLeftFloor _returnvalue)
  (bind _returnvalue_2 (Game|SpawnActorfromClass "/Game/Blueprints/BP_Floor.BP_Floor_C" _transformmid "Undefined" 0 2 true _self 0))
  (Variables|Default|SetCenterFloor _returnvalue_2)
  (bind _returnvalue_3 (Game|SpawnActorfromClass "/Game/Blueprints/BP_Floor.BP_Floor_C" _transformright "Undefined" 0 2 false _self 0))
  (Variables|Default|SetRightFloor _returnvalue_3)
  (CallFunction|ConstructLandingNodes)
  (if (Variables|Default|GetbCreateLogs)
    (CallFunction|ConstructInitialLogs)))

(event EventTick
  (params (DeltaSeconds :type Float%20%28single-precision%29))
  (|CallParentFunction DeltaSeconds)
  (if (Variables|Default|GetbCreateLogs)
    (CallFunction|ConstructLogAttempt DeltaSeconds))
  (CallFunction|CheckifDestroyFloorChunk))

(event EventDestroyed
  (for _array_element (Variables|Default|GetLilyPads)
    (Actor|DestroyActor _array_element)))

(fn ConstructionScript
  (|CallParentFunction)
  (if (Variables|Default|GetbCreateLogs)
    (Variables|Default|SetMaxCreateLogTime (Math|Random|RandomFloatinRange 0.0 1.0))
    (CallFunction|AddExtraLogSpeedRandom)))

(fn ConstructLilyPad
  (params (CurrentX :type Float%20%28single-precision%29))
  (bind _returnvalue (Transformation|GetActorLocation))
  (if (not (== CurrentX -1.0))
    (bind _returnvalue_2 (Game|SpawnActorfromClass "/Game/Blueprints/BP_LilyPad.BP_LilyPad_C" (Math|Transform|MakeTransform (Math|Vector|MakeVector CurrentX (.y _returnvalue) (- (.z _returnvalue) 3e+01))) "Undefined" 0 0))
    (Utilities|Array|Add (Variables|Default|GetLilyPads) _returnvalue_2)))

(fn ConstructLilyPads(Multiple)
  (bind _currentclearcolumpositionx3 (Variables|Default|GetCurrentClearColumPositionX3))
  (if (>= (Variables|Default|GetNumberOfLilyPadsToCreate) 1)
    (CallFunction|ConstructLilyPad (Variables|Default|GetCurrentClearColumPositionX1))
    (if (>= (Variables|Default|GetNumberOfLilyPadsToCreate) 2)
      (if (not (== (Variables|Default|GetCurrentClearColumPositionX1) (Variables|Default|GetCurrentClearColumPositionX2)))
        (CallFunction|ConstructLilyPad (Variables|Default|GetCurrentClearColumPositionX2))
        (if (>= (Variables|Default|GetNumberOfLilyPadsToCreate) 3)
          (if (not (or (== (Variables|Default|GetCurrentClearColumPositionX2) _currentclearcolumpositionx3) (== _currentclearcolumpositionx3 (Variables|Default|GetCurrentClearColumPositionX1))))
            (CallFunction|ConstructLilyPad (Variables|Default|GetCurrentClearColumPositionX3))))))))

(fn ConstructLandingNodes
  (Variables|Default|SetCurrentZPosForLandingNode -6e+01)
  (for _index (range 0 8)
    (CallFunction|ContructLandingNode(FloorChunk) true))
  (if (Variables|Default|GetbCreateLilyPads)
    (CallFunction|ConstructLilyPads(Multiple))))

(fn ConstructLog
  (params (LocationX :type Float%20%28single-precision%29))
  (bind _returnvalue (Transformation|GetActorLocation))
  (bind _returnvalue_2 (Game|SpawnActorfromClass "/Game/Blueprints/BP_Log.BP_Log_C" (Math|Transform|MakeTransform (Math|Vector|MakeVector LocationX (.y _returnvalue) (.z _returnvalue))) "Undefined" 0 (Math|Random|RandomIntegerinRange 1 3) (not (Variables|Default|GetbCreateLogsLeft)) (Variables|Default|GetExtraLogSpeedCenter) 0))
  (bind _output_get (Variables|Default|SetCurrentLogCreated _returnvalue_2))
  (return _output_get))

(fn CalculateLogCreationOffsetNext
  (Utilities|IsValid (Variables|Default|GetCurrentLogCreated)
    (:Is%20Valid
      (switch int (Variables|/Game/Blueprints/BP_Log.BP_Log_C|GetLength (Variables|Default|GetCurrentLogCreated))
        (:1
          (return (Math|Random|RandomFloatinRange 4e+02 5e+02)))
        (:2
          (return (Math|Random|RandomFloatinRange 6e+02 7e+02)))
        (:3
          (return (Math|Random|RandomFloatinRange 8e+02 9e+02)))))
    (:Is%20Not%20Valid
      (return (Math|Random|RandomFloatinRange 0.0 1e+02)))))

(fn ConstructInitialLogs
  (if (Variables|Default|GetbCreateLogsLeft)
    (LocalVariables|SetLogCreateXPos -9e+02)
    (while (< (LocalVariables|GetLogCreateXPos) 9e+02)
      (bind _randomxpos (CallFunction|CalculateLogCreationOffsetNext))
      (bind _output_get (LocalVariables|SetLogCreateXPos (+ _randomxpos (LocalVariables|GetLogCreateXPos))))
      (CallFunction|ConstructLog _output_get))
    (else
      (LocalVariables|SetLogCreateXPos 9e+02)
      (while (> (LocalVariables|GetLogCreateXPos) -9e+02)
        (bind _randomxpos_2 (CallFunction|CalculateLogCreationOffsetNext))
        (bind _output_get_2 (LocalVariables|SetLogCreateXPos (- (LocalVariables|GetLogCreateXPos) _randomxpos_2)))
        (CallFunction|ConstructLog _output_get_2)))))

(fn AddExtraLogSpeedRandom
  (Variables|Default|SetExtraLogSpeedCenter (Math|Random|RandomFloatinRange 0.0 2e+02)))

(fn ConstructLogAttempt
  (params (DeltaTime :type Float%20%28single-precision%29))
  (bind _extralogspeedcenter (Variables|Default|GetExtraLogSpeedCenter))
  (bind _returnvalue (/ _extralogspeedcenter 4e+02))
  (bind _output_get (Variables|Default|SetCurrentCreateLogTime (+ DeltaTime (Variables|Default|GetCurrentCreateLogTime))))
  (if (>= _output_get (Variables|Default|GetMaxCreateLogTime))
    (if (Variables|Default|GetbCreateLogsLeft)
      (CallFunction|ConstructLog -2.8e+03)
      (else
        (CallFunction|ConstructLog 2.8e+03)))
    (Variables|Default|SetCurrentCreateLogTime 0.0)
    (switch int (Variables|/Game/Blueprints/BP_Log.BP_Log_C|GetLength (Variables|Default|GetCurrentLogCreated))
      (:1
        (Variables|Default|SetMaxCreateLogTime (- (Math|Random|RandomFloatinRange 1.25 1.5) _returnvalue)))
      (:2
        (Variables|Default|SetMaxCreateLogTime (- (Math|Random|RandomFloatinRange 1.5 1.75) _returnvalue)))
      (:3
        (Variables|Default|SetMaxCreateLogTime (- (Math|Random|RandomFloatinRange 2.0 2.25) _returnvalue))))))