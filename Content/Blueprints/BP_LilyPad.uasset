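; BP_LilyPad is a lily pad that the chicken lands on, bouncing and slowly turning while occupied.
; On BeginPlay it picks a random yaw spin rate, rolls a random integer and has logic to spawn a coin at its location.
; Tick plays a sound as a jump landing begins, runs the bounce animation and applies the spin only while a chicken is on top.
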(event EventBeginPlay
  (|CallParentFunction)
  (Variables|Default|SetRotation (Math|Rotator|MakeRotator 0.0 0.0 (Math|Random|RandomFloatinRange -2e+01 2e+01)))
  (switch int (Math|Random|RandomInteger 3)
    (:Default
      (Game|SpawnActorfromClass "/Game/Blueprints/BP_Coin.BP_Coin_C" (Math|Transform|MakeTransform (Transformation|GetActorLocation)) "Undefined" 0 0))))

(event Collision|EventActorBeginOverlap
  (params (OtherActor :type Actor%20Object%20Reference)))

(event EventTick
  (params (DeltaSeconds :type Float%20%28single-precision%29))
  (CallFunction|AttemptPlayJumpedonSound)
  (CallFunction|BouncingAnimation DeltaSeconds)
  (if (Variables|Default|GetbHasChickenOnTop)
    (Transformation|AddActorLocalRotation (* (Variables|Default|GetRotation) DeltaSeconds) false false)))

(fn ConstructionScript
  (|CallParentFunction))

(fn AttemptPlayJumpedonSound
  (if (and (== (Variables|Default|GetCurrentJumpedOnTime) 0.0) (Variables|Default|GetbIsBeingJumpedOn))
    (Audio|PlaySound2D "/Game/media/sounds/lily_pad.lily_pad" 1.0 1.0 0.0 0 0)))