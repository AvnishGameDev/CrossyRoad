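; Crossy Road-style game mode that sets the camera view, builds the starting lanes and reloads the level after game over.
; First Tick spawns opening grass, then random grass, road, water and railroad chunks, avoiding repeated types.
; Shared clear-column positions feed grass and water rows, which choose logs or lily pads.
; Chunk length tightens with forward progress, but Tick's ongoing ConstructFloors call is unwired and CreateUI is empty.
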(event EventBeginPlay
  (bind _returnvalue (Game|GetPlayerController 0))
  (CallFunction|CreateUI)
  (Input|EnableInput _returnvalue 0)
  (Variables|/Script/Engine.PlayerController|SetbShowMouseCursor _returnvalue true)
  (Variables|Default|SetbCanRunProgram true)
  (bind _outactors (Actor|GetAllActorswithTag "Camera"))
  (for _array_element _outactors
    (bind _asbp_main_camera (Utilities|Casting|CastToBP_Main_Camera _array_element))
    (bind _output_get (Variables|Default|SetCameraRef _asbp_main_camera))
    (Game|Player|SetViewTargetwithBlend (Game|GetPlayerController 0) _output_get 0.0 "VTBlend_Linear" 0.0 false)))

(event EventTick
  (params (DeltaSeconds :type Float%20%28single-precision%29))
  (if (Variables|Default|GetbCanRunProgram)
    (if (Variables|Default|GetbConstructedInitialFloorChunks)
      (if (Variables|Default|GetbGameOver)
        (Variables|Default|SetbGameOver false)
        (Utilities|FlowControl|Delay 3.0)
        (Game|OpenLevel(byName) "Main"))
      (else
        (CallFunction|ConstructInitialFloors)
        (Variables|Default|SetbConstructedInitialFloorChunks true)))))

(fn ConstructionScript)

(fn CreateClearColumnPositions
  (Variables|Default|SetClearColumnPositionX1 -1.0)
  (Variables|Default|SetClearColumnPositionX2 -1.0)
  (Variables|Default|SetClearColumnPositionX3 -1.0)
  (for _index (range 0 (Math|Random|RandomInteger 2))
    (switch int _index
      (:0
        (Variables|Default|SetClearColumnPositionX1 (- (* (Math|Random|RandomInteger 8) 2e+02) 8e+02))))))

(fn CalculateFloorSpawnY
  (return (- (* (Variables|Default|GetCurrentFloorIndex) (Variables|Default|GetFloorSpawnYDelta)) 2e+02)))

(fn CreateGrassFloorChunk
  (params (NumberOfFloors :type Integer) (bCenterClearColumn :type Boolean))
  (if (== (Variables|Default|GetPreviousFloorTypeCreated) 2)
    _
    (else
      (CallFunction|CreateClearColumnPositions)))
  (if bCenterClearColumn
    (Variables|Default|SetClearColumnPositionX3 0.0))
  (for _index (range 0 (- NumberOfFloors 1))
    (Variables|Default|SetCurrentFloorIndex (+ (Variables|Default|GetCurrentFloorIndex) 1))
    (bind _postiony (CallFunction|CalculateFloorSpawnY))
    (Game|SpawnActorfromClass "/Game/Blueprints/BP_Grass.BP_Grass_C" (Math|Transform|MakeTransform (Math|Vector|MakeVector 0.0 _postiony 0.0)) "Undefined" 0 (not (== (Math|Integer|%(Integer) _index 2) 0)) (Variables|Default|GetClearColumnPositionX1) (Variables|Default|GetClearColumnPositionX2) (Variables|Default|GetClearColumnPositionX3) (Variables|Default|GetChickenRef) _postiony 0)))

(fn CalculateCurrentFloorTypetoCreate
  (Variables|Default|SetPreviousFloorTypeCreated (Variables|Default|GetCurrentFloorTypeCreated))
  (Variables|Default|SetCurrentFloorTypeCreated (Math|Random|RandomInteger 4))
  (if (== (Variables|Default|GetCurrentFloorTypeCreated) (Variables|Default|GetPreviousFloorTypeCreated))
    (switch int (Variables|Default|GetPreviousFloorTypeCreated)
      (:0
        (Variables|Default|SetCurrentFloorTypeCreated 1))
      (:1
        (Variables|Default|SetCurrentFloorTypeCreated 2))
      (:2
        (Variables|Default|SetCurrentFloorTypeCreated 3))
      (:3
        (Variables|Default|SetCurrentFloorTypeCreated 0)))))

(fn CreateRoadFloorChunk
  (params (NumberOfFloorsToCreate :type Integer))
  (for _index (range 0 (- NumberOfFloorsToCreate 1))
    (Variables|Default|SetCurrentFloorIndex (+ (Variables|Default|GetCurrentFloorIndex) 1))
    (bind _postiony (CallFunction|CalculateFloorSpawnY))
    (Game|SpawnActorfromClass "/Game/Blueprints/BP_Road.BP_Road_C" (Math|Transform|MakeTransform (Math|Vector|MakeVector 0.0 _postiony 0.0)) "Undefined" 0 (>= _index 1) (Variables|Default|GetChickenRef) _postiony 0)))

(fn CreateRailroadFloorChunk
  (params (NumberOfFloors :type Integer))
  (for _index (range 0 (- NumberOfFloors 1))
    (Variables|Default|SetCurrentFloorIndex (+ (Variables|Default|GetCurrentFloorIndex) 1))
    (bind _postiony (CallFunction|CalculateFloorSpawnY))
    (Game|SpawnActorfromClass "/Game/Blueprints/BP_Railroad.BP_Railroad_C" (Math|Transform|MakeTransform (Math|Vector|MakeVector 0.0 _postiony 0.0)) "Undefined" 0 (Variables|Default|GetChickenRef) _postiony 0)))

(fn CountNumberOfLillyPadstoCreate
  (Variables|Default|SetNumberOfLillyPadsToCreate 0)
  ;[1 1 1] Clear Column X1
  (if (!= (Variables|Default|GetClearColumnPositionX1) -1.0)
    (Variables|Default|SetNumberOfLillyPadsToCreate (+ (Variables|Default|GetNumberOfLillyPadsToCreate) 1)))
  ;[1 1 1] Clear Column X2
  (if (!= (Variables|Default|GetClearColumnPositionX2) -1.0)
    (Variables|Default|SetNumberOfLillyPadsToCreate (+ (Variables|Default|GetNumberOfLillyPadsToCreate) 1)))
  ;[1 1 1] Clear Column X3
  (if (!= (Variables|Default|GetClearColumnPositionX3) -1.0)
    (Variables|Default|SetNumberOfLillyPadsToCreate (+ (Variables|Default|GetNumberOfLillyPadsToCreate) 1))))

(fn CreateWaterFloorChunk
  (params (NumberOfFloors :type Integer))
  (for _index (range 0 (- NumberOfFloors 1))
    (Variables|Default|SetCurrentFloorIndex (+ (Variables|Default|GetCurrentFloorIndex) 1))
    (bind _postiony (CallFunction|CalculateFloorSpawnY))
    (if (== (Math|Random|RandomIntegerinRange 0 4) 0)
      (if (Variables|Default|GetbCanCreateLilyPads)
        ;[1 1 1] Can Create Lilly Pads
        (if (Variables|Default|GetbCreatedLillyPadsSinceWaterChunkGroupStarted)
          (CallFunction|CreateClearColumnPositions))
        (CallFunction|CountNumberOfLillyPadstoCreate)
        (Game|SpawnActorfromClass "/Game/Blueprints/BP_Water.BP_Water_C" (Math|Transform|MakeTransform (Math|Vector|MakeVector 0.0 _postiony 0.0)) "Undefined" 0 false false true (Variables|Default|GetNumberOfLillyPadsToCreate) (Variables|Default|GetClearColumnPositionX1) (Variables|Default|GetClearColumnPositionX2) (Variables|Default|GetClearColumnPositionX3) (Variables|Default|GetChickenRef) _postiony 0)
        (Variables|Default|SetbCreatedLillyPadsSinceWaterChunkGroupStarted true)
        (Variables|Default|SetbCanCreateLilyPads false)
        (Variables|Default|SetbCreatedLeftLogsSinceLillyPads false)
        (Variables|Default|SetbCreatedRightLogsSinceLillyPads false)
        (else
          ;[1 1 1] Can't Create Lilly Pads
          (bind _output_get (Variables|Default|SetbCreateLogsLeft (Math|Random|RandomBool) :!label _label))
          (if (Math|Boolean|Equal(Boolean) _output_get (Variables|Default|GetbPreviousLogCreationDirection))
            (bind _output_get_2 (Variables|Default|SetNumberOfLogsCreatedInSameDirection (+ (Variables|Default|GetNumberOfLogsCreatedInSameDirection) 1)))
            (if (> _output_get_2 2)
              (bind _output_get_3 (Variables|Default|SetbCreateLogsLeft (not (Variables|Default|GetbCreateLogsLeft))))
              (Variables|Default|SetNumberOfLogsCreatedInSameDirection 0)
              (Variables|Default|SetbPreviousLogCreationDirection _output_get_3))
            (else
              (Variables|Default|SetNumberOfLogsCreatedInSameDirection 1)))
          (Game|SpawnActorfromClass "/Game/Blueprints/BP_Water.BP_Water_C" (Math|Transform|MakeTransform (Math|Vector|MakeVector 0.0 _postiony 0.0)) "Undefined" 0 true (Variables|Default|GetbCreateLogsLeft) false 0 (Variables|Default|GetClearColumnPositionX1) (Variables|Default|GetClearColumnPositionX2) (Variables|Default|GetClearColumnPositionX3) (Variables|Default|GetChickenRef) _postiony 0)
          (if (Variables|Default|GetbCreateLogsLeft)
            (Variables|Default|SetbCreatedLeftLogsSinceLillyPads true)
            (else
              (Variables|Default|SetbCreatedRightLogsSinceLillyPads false)))
          (if (Variables|Default|GetbCreatedLeftLogsSinceLillyPads)
            (if (Variables|Default|GetbCreatedRightLogsSinceLillyPads)
              (Variables|Default|SetbCanCreateLilyPads true)))
          (Variables|Default|SetbPreviousLogCreationDirection (Variables|Default|GetbCreateLogsLeft))))
      (else
        (goto _label)))))

(fn ConstructFloors
  (bind _numberchunksexploredforward (Variables|Default|GetNumberChunksExploredForward))
  (bind _numberchunksexploredforward_2 (Variables|Default|GetNumberChunksExploredForward))
  (bind _returnvalue (/ _numberchunksexploredforward_2 20))
  (bind _returnvalue_2 (/ _numberchunksexploredforward 20))
  (bind _returnvalue_3 (- 6 _returnvalue))
  (bind _returnvalue_4 (- 6 _returnvalue_2))
  (bind _returnvalue_5 (Math|Random|RandomInteger _returnvalue_3))
  (bind _returnvalue_6 (Math|Random|RandomInteger _returnvalue_4))
  (bind _returnvalue_7 (+ _returnvalue_6 1))
  (bind _returnvalue_8 (+ _returnvalue_5 1))
  (while (< (- (Variables|Default|GetCurrentFloorIndex) (Variables|Default|GetPlayerPositionIndex)) 20)
    (CallFunction|CalculateCurrentFloorTypetoCreate)
    (switch int (Variables|Default|GetCurrentFloorTypeCreated)
      (:0
        (if (< _returnvalue_8 1)
          (CallFunction|CreateGrassFloorChunk _returnvalue_8 false)
          (else
            (CallFunction|CreateGrassFloorChunk 1 false))))
      (:1
        (CallFunction|CreateRoadFloorChunk _returnvalue_7))
      (:2
        (Variables|Default|SetbCreatedLillyPadsSinceWaterChunkGroupStarted false)
        (CallFunction|CreateWaterFloorChunk _returnvalue_7))
      (:3
        (CallFunction|CreateRailroadFloorChunk _returnvalue_7)))))

(fn ConstructInitialFloors
  (CallFunction|CreateGrassFloorChunk 8 true)
  (CallFunction|CreateGrassFloorChunk 2 true)
  (CallFunction|ConstructFloors))

(fn CreateUI)