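; Vehicle spawner for a lane in a chicken-crossing game, passing a random per-spawner speed, its facing and the chicken reference to each BP_Vehicle.
; Tick spawns a vehicle at the spawner whenever a randomly re-rolled timer expires.
; BeginPlay also runs a pre-fill loop while ContinueCreatingVehicles holds, spawning at one fixed X offset set by facing.
; That loop computes random spacing but never applies it to spawn positions or updates its flag here.
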(event EventBeginPlay
  (Variables|Default|SetSpeed (Math|Random|RandomFloatinRange 3e+02 6e+02))
  (CallFunction|SetNewMaxTimeforSpawn)
  (CallFunction|SpawnInitialVehicles))

(event EventTick
  (params (DeltaSeconds :type Float%20%28single-precision%29))
  (bind _output_get (Variables|Default|SetTimeAccumilation (+ DeltaSeconds (Variables|Default|GetTimeAccumilation))))
  (if (>= _output_get (Variables|Default|GetTimeMaxForSpawn))
    (Variables|Default|SetTimeAccumilation 0.0)
    (CallFunction|SetNewMaxTimeforSpawn)
    (Game|SpawnActorfromClass "/Game/Blueprints/BP_Vehicle.BP_Vehicle_C" (Transformation|GetActorTransform) "Undefined" 0 (Variables|Default|GetbFacingLeft) (Variables|Default|GetSpeed) (Variables|Default|GetChickenRef) 0)))

(fn ConstructionScript)

(fn SetNewMaxTimeforSpawn
  (Variables|Default|SetTimeMaxForSpawn (Math|Random|RandomFloatinRange 2.0 5.0)))

(fn SpawnInitialVehicles
  (bind _returnvalue (Transformation|GetActorLocation))
  (bind _returnvalue_2 (Math|Random|RandomFloatinRange 6e+02 1.2e+03))
  (bind _returnvalue_3 (Transformation|GetActorLocation))
  (if (Variables|Default|GetbFacingLeft)
    (LocalVariables|SetXOffsetInitial (+ (.x _returnvalue) -6e+02))
    (else
      (LocalVariables|SetXOffsetInitial (+ (.x _returnvalue) 6e+02))))
  (while (LocalVariables|GetbContinueCreatingVehicles)
    (LocalVariables|SetXOffsetAccumilation _returnvalue_2)
    (LocalVariables|SetDistanceAccumilation (+ _returnvalue_2 (LocalVariables|GetDistanceAccumilation)))
    (if (Variables|Default|GetbFacingLeft)
      (LocalVariables|SetXOffsetAccumilation (* (LocalVariables|GetXOffsetAccumilation) -1.0)))
    (Game|SpawnActorfromClass "/Game/Blueprints/BP_Vehicle.BP_Vehicle_C" (Math|Transform|MakeTransform (Math|Vector|MakeVector (LocalVariables|GetXOffsetInitial) (.y _returnvalue_3) (.z _returnvalue_3))) "Undefined" 0 (Variables|Default|GetbFacingLeft) (Variables|Default|GetSpeed) (Variables|Default|GetChickenRef) 0)))