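; Floor tile for a chicken player game that becomes grass, road or water based on FloorType.
; BeginPlay sets the mesh and collision: grass and road block, water overlaps.
; A chicken player overlapping water spawns splashes and triggers its game-over sequence.
; Non-traversable tiles call DarkenMesh on a dynamic material, though it reads "darkness" and writes to parameter "None".
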(event Custom|OnComponentBeginOverlap_Event_0
  (params (OverlappedComponent :type Primitive%20Component%20Object%20Reference) (OtherActor :type Actor%20Object%20Reference) (OtherComp :type Primitive%20Component%20Object%20Reference) (OtherBodyIndex :type Integer) (bFromSweep :type Boolean) (SweepResult :type Hit%20Result%20Structure%20%28by%20ref%29))
  (bind _asbp_chicken_player (Utilities|Casting|CastToBP_Chicken_Player OtherActor))
  (if (== (Variables|Default|GetFloor%20Type) 2)
    (for _index (range 0 2)
      (Game|SpawnActorfromClass "/Game/Blueprints/BP_Water_Splash.BP_Water_Splash_C" (Math|Transform|MakeTransform (Math|Vector|MakeVector (.x (Transformation|GetActorLocation _asbp_chicken_player)) (.y (Transformation|GetActorLocation _asbp_chicken_player)) (+ (.z (Transformation|GetActorLocation _asbp_chicken_player)) 1e+01))) "Undefined" 0 0)
      (Default|GameOverSequence _asbp_chicken_player))))

(event EventBeginPlay
  (bind _waterbox (Variables|Default|GetWaterBox))
  (bind _grassbox (Variables|Default|GetGrassBox))
  (Collision|AssignOnComponentBeginOverlap (Variables|Default|GetWaterBox) (delegate Custom|OnComponentBeginOverlap_Event_0))
  (Utilities|FlowControl|MultiGate false false (Variables|Default|GetFloor%20Type)
    (:Out%200
      (CallFunction|SetMesh "/Game/media/meshes/grass.grass")
      (Collision|SetCollisionEnabled _grassbox "QueryAndPhysics" :!label _label)
      (Collision|SetCollisionResponsetoAllChannels _grassbox "ECR_Block"))
    (:Out%201
      (CallFunction|SetMesh "/Game/media/meshes/road.road")
      (goto _label))
    (:Out%202
      (CallFunction|SetMesh "/Game/media/meshes/water.water")
      (Collision|SetCollisionEnabled _waterbox "QueryOnly")
      (Collision|SetCollisionResponsetoAllChannels _waterbox "ECR_Overlap"))))

(event Collision|EventActorBeginOverlap
  (params (OtherActor :type Actor%20Object%20Reference))
  (bind _asbp_chicken_player (Utilities|Casting|CastToBP_Chicken_Player (stale Custom|OnComponentBeginOverlap_Event_0 OtherActor)))
  (if (== (Variables|Default|GetFloor%20Type) 2)
    (for _index (range 0 2)
      (Game|SpawnActorfromClass "/Game/Blueprints/BP_Water_Splash.BP_Water_Splash_C" (Math|Transform|MakeTransform (Math|Vector|MakeVector (.x (Transformation|GetActorLocation _asbp_chicken_player)) (.y (Transformation|GetActorLocation _asbp_chicken_player)) (+ (.z (Transformation|GetActorLocation _asbp_chicken_player)) 1e+01))) "Undefined" 0 0)
      (Default|GameOverSequence _asbp_chicken_player))))

(fn ConstructionScript)

(fn DarkenMesh
  (params (MaterialInstance :type Material%20Instance%20Dynamic%20Object%20Reference))
  (bind _returnvalue (Rendering|Material|GetVectorParameterValue MaterialInstance "darkness" :!class /Script/Engine.MaterialInstanceDynamic))
  (Rendering|Material|SetVectorParameterValue MaterialInstance "None" (Math|Conversions|ToLinearColor(Float) (- (.R (Utilities|Struct|BreakLinearColor _returnvalue)) 0.4)) :!class /Script/Engine.MaterialInstanceDynamic))

(fn SetMesh
  (params (Static%20Mesh :type Static%20Mesh%20Object%20Reference))
  (bind _floormesh (Variables|Default|GetFloorMesh))
  (Components|StaticMesh|SetStaticMesh _floormesh Static%20Mesh)
  (bind _returnvalue (Rendering|Material|CreateDynamicMaterialInstance _floormesh 0 "/Game/media/meshes/M_chicken__colors_png.M_chicken__colors_png" "None" :!class /Script/Engine.PrimitiveComponent))
  (bind _output_get (Variables|Default|SetMaterialInstance _returnvalue))
  (if (not (Variables|Default|GetTraversable))
    (CallFunction|DarkenMesh _output_get)))